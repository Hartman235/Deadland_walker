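; Actor component on the player character that spawns mutant zombies on a repeating timer and in periodic waves.
; A second timer increments Wave and loops over a growing count, with a short Delay before each Spawn call.
; Spawn places zombies at a set Distance along the owner's velocity, or forward vector when still, rotated by owner yaw.
; Each zombie's death event is forwarded to Bp_GameState's OnKill.
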(event Custom|OnKill
  (bind _asbp_game_state (Utilities|Casting|CastToBp_GameState (Game|GetGameState)))
  (Default|OnKill _asbp_game_state))

(event Custom|SpawnZombie
  (CallFunction|Spawn))

(event Custom|Spawn
  (bind _returnvalue (Components|GetOwner))
  (bind _distance (Variables|Default|GetDistance))
  (bind _asbp_third_person_character (Utilities|Casting|CastToBP_ThirdPersonCharacter _returnvalue))
  (Development|PrintString "Zombie spawn attempt")
  (bind _returnvalue_2 (Game|SpawnActorfromClass "/Game/Zombie_Mutant/blueprint/BP_Zombie_Mutant_Blueprint.BP_Zombie_Mutant_Blueprint_C" (Math|Conversions|ToTransform(Vector) (+ (Transformation|GetActorLocation _returnvalue) (Math|Vector|RotateVector (Math|Vector|ClampVectorSize (Math|Vector|SelectVector (Class|KismetMathLibrary|VectorForward) (Variables|/Script/Engine.MovementComponent|GetVelocity (Variables|/Script/Engine.Character|GetCharacterMovement _asbp_third_person_character)) (Utilities|Operators|EqualEqual :A (Variables|/Script/Engine.MovementComponent|GetVelocity (Variables|/Script/Engine.Character|GetCharacterMovement _asbp_third_person_character)) :ErrorTolerance 0.1)) _distance _distance) (Math|Rotator|MakeRotator 0.0 0.0 (.yaw (Transformation|GetActorRotation _returnvalue)))) (Math|Vector|MakeVector (Math|Random|RandomFloatinRange 0.0 0.0) (Math|Random|RandomFloatinRange 0.0 0.0) 0.0))) "AdjustIfPossibleButAlwaysSpawn" "MultiplyWithRoot" 0 0))
  (EventDispatchers|BindEventtoOnDead (Variables|/Game/Zombie_Mutant/blueprint/BP_Zombie_Mutant_Blueprint.BP_Zombie_Mutant_Blueprint_C|GetHealth_component _returnvalue_2) (delegate Custom|OnKill))
  (Development|PrintString "Zombie spawn"))

(event Custom|SpawnWave
  (bind _result (Math|Integer|IncrementInt (Variables|Default|Getwave))
    (:%20%20
      (bind _output_get (Variables|Default|Setwave _result))
      (for _index (range 0 (+ (* _output_get 2) 3))
        (Utilities|FlowControl|Delay 0.1)
        (CallFunction|Spawn)))))

(event EventBeginPlay
  (Utilities|Time|SetTimerbyEvent (delegate Custom|SpawnZombie) (Variables|Default|GetSeconds) true)
  (Utilities|Time|SetTimerbyEvent (delegate Custom|SpawnWave) (Variables|Default|Getwaveseconds) true))