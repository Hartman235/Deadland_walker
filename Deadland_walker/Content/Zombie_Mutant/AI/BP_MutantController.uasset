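; AI controller for the mutant zombie that runs the BT_Mutant behavior tree and feeds its perception into the blackboard.
; Perception updates from other mutants are ignored; the rest pass to separate sight, hearing and prediction handlers.
; Sight sets TargetActor, or clears it on loss and requests a short prediction of where that actor is heading.
; Successful hearing and prediction stimuli write their location to LastKnownLocation.
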(event OnTargetPerceptionUpdated(AIPerception)
  (params (Actor :type Actor%20Object%20Reference) (Stimulus :type AI%20Stimulus%20Structure))
  (Utilities|Casting|CastToBP_Zombie_Mutant_Blueprint Actor
    (:CastFailed
      (CallFunction|HandleSightSense Actor Stimulus)
      (CallFunction|HandleHearingSense Stimulus)
      (CallFunction|HandlePredictionSense Stimulus))))

(event EventBeginPlay
  (AI|RunBehaviorTree "/Game/Zombie_Mutant/AI/BT_Mutant.BT_Mutant"))

(fn ConstructionScript)

(fn HandleSightSense
  (params (Actor :type Actor%20Object%20Reference) (Stimulus :type AI%20Stimulus%20Structure))
  (bind _returnvalue (Class|AIPerceptionSystem|GetSenseClassforStimulus Stimulus))
  (if (== _returnvalue "/Script/AIModule.AISense_Sight")
    (if (.bSuccessfullySensed (Utilities|Struct|BreakAIStimulus Stimulus))
      (AI|Components|Blackboard|SetValueasObject (Variables|Default|GetBlackboard) (Utilities|Name|MakeLiteralName "TargetActor") Actor)
      (else
        (AI|Components|Blackboard|SetValueasObject (Variables|Default|GetBlackboard) (Utilities|Name|MakeLiteralName "TargetActor") 0)
        (Class|AISensePrediction|RequestControllerPredictionEvent self Actor 0.5)))))

(fn HandleHearingSense
  (params (Stimulus :type AI%20Stimulus%20Structure))
  (bind (_age _expirationage _strength _stimuluslocation _receiverlocation _tag _bsuccessfullysensed) (Utilities|Struct|BreakAIStimulus Stimulus))
  (bind _returnvalue (Class|AIPerceptionSystem|GetSenseClassforStimulus Stimulus))
  (if (== _returnvalue "/Script/AIModule.AISense_Hearing")
    (if _bsuccessfullysensed
      (AI|Components|Blackboard|SetValueasVector (Variables|Default|GetBlackboard) (Utilities|Name|MakeLiteralName "LastKnownLocation") _stimuluslocation))))

(fn HandlePredictionSense
  (params (Stimulus :type AI%20Stimulus%20Structure))
  (bind (_age _expirationage _strength _stimuluslocation _receiverlocation _tag _bsuccessfullysensed) (Utilities|Struct|BreakAIStimulus Stimulus))
  (bind _returnvalue (Class|AIPerceptionSystem|GetSenseClassforStimulus Stimulus))
  (if (== _returnvalue "/Script/AIModule.AISense_Prediction")
    (if _bsuccessfullysensed
      (AI|Components|Blackboard|SetValueasVector (Variables|Default|GetBlackboard) (Utilities|Name|MakeLiteralName "LastKnownLocation") _stimuluslocation))))