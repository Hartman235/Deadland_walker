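; AI character for what appears to be a game of tag, with patrol points and contact-based swapping of a Tagged gameplay tag.
; On BeginPlay it stores its spawn location as AnchorPoint and offsets each PatrolPoints entry by it, turning relative points into world positions.
; When its Box overlaps BP_ThirdPersonCharacter, it hands Tagged to that character if it holds it, otherwise takes it and clears the character's.
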(event OnComponentBeginOverlap(Box)
  (params (OverlappedComponent :type Primitive%20Component%20Object%20Reference) (OtherActor :type Actor%20Object%20Reference) (OtherComp :type Primitive%20Component%20Object%20Reference) (OtherBodyIndex :type Integer) (bFromSweep :type Boolean) (SweepResult :type Hit%20Result%20Structure%20%28by%20ref%29))
  (bind _gameplaytags (Variables|Default|GetGameplayTags))
  (bind _asbp_third_person_character (Utilities|Casting|CastToBP_ThirdPersonCharacter OtherActor))
  (if (GameplayTags|HasTag (Variables|Default|GetGameplayTags) "(TagName=\"Tagged\")" true)
    (GameplayTags|RemoveGameplayTag _gameplaytags "(TagName=\"Tagged\")" :!class /Script/GameplayTags.BlueprintGameplayTagLibrary)
    (GameplayTags|AddGameplayTag (Variables|/Game/ThirdPerson/Blueprints/BP_ThirdPersonCharacter.BP_ThirdPersonCharacter_C|GetGameplayTags _asbp_third_person_character) "(TagName=\"Tagged\")" :!class /Script/GameplayTags.BlueprintGameplayTagLibrary)
    (else
      (GameplayTags|AddGameplayTag _gameplaytags "(TagName=\"Tagged\")" :!class /Script/GameplayTags.BlueprintGameplayTagLibrary)
      (GameplayTags|RemoveGameplayTag (Variables|/Game/ThirdPerson/Blueprints/BP_ThirdPersonCharacter.BP_ThirdPersonCharacter_C|GetGameplayTags _asbp_third_person_character) "(TagName=\"Tagged\")" :!class /Script/GameplayTags.BlueprintGameplayTagLibrary))))

(event EventBeginPlay
  (Variables|Default|SetAnchorPoint (Transformation|GetActorLocation))
  (for (_array_element _array_index) (Variables|Default|GetPatrolPoints)
    (Utilities|Array|SetArrayElem (Variables|Default|GetPatrolPoints) _array_index (+ _array_element (Variables|Default|GetAnchorPoint)))))

(fn ConstructionScript)