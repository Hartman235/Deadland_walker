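; Spawner actor that creates one mutant zombie at its own location on BeginPlay and can report kills to the game state.
; SpawnZombieInRadius always spawns the zombie, adjusting for collision if possible, and binds an event to its HealthComponent's OnDead; the Radius input is unused.
; OnKill forwards to Bp_GameState's OnKill.
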(event Custom|OnKill
  (bind _asbp_game_state (Utilities|Casting|CastToBp_GameState (Game|GetGameState)))
  (Default|OnKill _asbp_game_state))

(event EventBeginPlay
  (CallFunction|SpawnZombieinRadius 0.0))

(event Collision|EventActorBeginOverlap
  (params (OtherActor :type Actor%20Object%20Reference)))

(event EventTick
  (params (DeltaSeconds :type Float%20%28single-precision%29)))

(fn ConstructionScript)

(fn SpawnZombieinRadius
  (params (Radius :type Float%20%28double-precision%29))
  (bind _returnvalue (Game|SpawnActorfromClass "/Game/Zombie_Mutant/blueprint/BP_Zombie_Mutant_Blueprint.BP_Zombie_Mutant_Blueprint_C" (Math|Conversions|ToTransform(Vector) (Transformation|GetActorLocation)) "AdjustIfPossibleButAlwaysSpawn" "MultiplyWithRoot" 0 0))
  (EventDispatchers|BindEventtoOnDead (Variables|/Game/Zombie_Mutant/blueprint/BP_Zombie_Mutant_Blueprint.BP_Zombie_Mutant_Blueprint_C|GetHealth_component _returnvalue) (EventDispatchers|CreateEvent :!event Custom|OnKill))
  (return _returnvalue))