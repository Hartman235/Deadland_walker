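; Zombie mutant enemy that deals repeated melee damage to nearby actors and ragdolls on death.
; Box overlap with an actor of another class that has a Health_component starts a Delay-based loop, applying damage until overlap ends or the zombie dies.
; Its own Health_component's OnDead event sets IsDead and enables mesh physics.
; A timeline-driven "Breath" morph target is present but never runs.
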(event OnDead(Health_component)
  (Variables|Default|SetisDead true)
  (Physics|SetSimulatePhysics (Variables|Character|GetMesh) true)
  (Development|PrintString "Zombie Death"))

(event Custom|BeginOverlap
  (params (OverlappedComponent :type Primitive%20Component%20Object%20Reference) (OtherActor :type Actor%20Object%20Reference) (OtherComp :type Primitive%20Component%20Object%20Reference) (OtherBodyIndex :type Integer) (bFromSweep :type Boolean) (SweepResult :type Hit%20Result%20Structure%20%28by%20ref%29))
  (bind _returnvalue (Actor|GetComponentbyClass OtherActor "/Game/Components/Health_component.Health_component_C"))
  (if (not (== (Utilities|GetClass OtherActor) (Utilities|GetClass self)))
    (Utilities|IsValid _returnvalue
      (:Is%20Valid
        (Variables|Default|SetIsAttacking true)
        (bind _output_get (Variables|Default|SetAttaclingActorHealthComp _returnvalue))
        (if (Variables|Default|GetIsAttacking) :!label _label
          (Utilities|FlowControl|Delay 0.2)
          (if (not (Variables|Default|GetIsDead))
            (Default|GetDamage _output_get 1e+01)
            (goto _label)))))))

(event Custom|EndOverlap
  (params (OverlappedComponent :type Primitive%20Component%20Object%20Reference) (OtherActor :type Actor%20Object%20Reference) (OtherComp :type Primitive%20Component%20Object%20Reference) (OtherBodyIndex :type Integer))
  (Variables|Default|SetIsAttacking false))

(event EventBeginPlay
  (bind _box (Variables|Default|GetBox))
  (Variables|Default|SetMaxSpeed (Variables|Default|GetMaxSpeed))
  (Collision|BindEventtoOnComponentBeginOverlap _box (delegate Custom|BeginOverlap))
  (Collision|BindEventtoOnComponentEndOverlap _box (delegate Custom|EndOverlap)))

(event Collision|EventActorBeginOverlap
  (params (OtherActor :type Actor%20Object%20Reference)))

(event EventTick
  (params (DeltaSeconds :type Float%20%28single-precision%29)))

(fn ConstructionScript)