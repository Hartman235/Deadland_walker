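; Actor component that repeatedly spawns mutant zombies in front of its owning actor.
; BeginPlay starts a looping timer with a configurable Seconds interval that fires SpawnZombie.
; Each spawn is placed Distance units from the owner's location along its yaw-only facing.
; Collision handling nudges the spawn point when possible but always spawns the zombie.
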(event Custom|SpawnZombie
  (bind _returnvalue (Components|GetOwner))
  (bind _distance (Variables|Default|GetDistance))
  (Game|SpawnActorfromClass "/Game/Zombie_Mutant/blueprint/BP_Zombie_Mutant_Blueprint.BP_Zombie_Mutant_Blueprint_C" (Math|Conversions|ToTransform(Vector) (+ (Transformation|GetActorLocation _returnvalue) (Math|Vector|RotateVector (Math|Vector|ClampVectorSize (Class|KismetMathLibrary|VectorForward) _distance _distance) (Math|Rotator|MakeRotator 0.0 0.0 (.yaw (Transformation|GetActorRotation _returnvalue)))))) "AdjustIfPossibleButAlwaysSpawn" "MultiplyWithRoot" 0 0))

(event EventBeginPlay
  (Utilities|Time|SetTimerbyEvent (delegate Custom|SpawnZombie) (Variables|Default|GetSeconds) true))