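; Barn map actor that periodically spawns zombies through a child zombie spawner while the player is outside its box volume.
; Box overlap events track player presence, and a looping timer requests a spawn in a radius while the live count is below capacity.
; Each zombie's health component death event decrements the count.
; An invalid spawn result triggers an immediate recursive retry.
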(event Custom|OnComponentEndOverlap_Event
  (params (OverlappedComponent :type Primitive%20Component%20Object%20Reference) (OtherActor :type Actor%20Object%20Reference) (OtherComp :type Primitive%20Component%20Object%20Reference) (OtherBodyIndex :type Integer))
  (Utilities|Casting|CastToBP_ThirdPersonCharacter OtherActor)
  (Variables|Default|SetIsPlayerInside false))

(event Custom|OnBeginOverlap
  (params (OverlappedComponent :type Primitive%20Component%20Object%20Reference) (OtherActor :type Actor%20Object%20Reference) (OtherComp :type Primitive%20Component%20Object%20Reference) (OtherBodyIndex :type Integer) (bFromSweep :type Boolean) (SweepResult :type Hit%20Result%20Structure%20%28by%20ref%29))
  (Utilities|Casting|CastToBP_ThirdPersonCharacter OtherActor)
  (Variables|Default|SetIsPlayerInside true))

(event Custom|TrySpawnMob
  (if (not (Variables|Default|GetIsPlayerInside))
    (if (< (Variables|Default|GetMobCount) (Variables|Default|GetMobCapacity))
      (bind _asbp_zombie_spawner (Utilities|Casting|CastToBp_ZombieSpawner (Variables|/Script/Engine.ChildActorComponent|GetChildActor (Variables|Default|GetBp_ZombieSpavner))))
      (bind _zombie (Default|SpawnZombieinRadius _asbp_zombie_spawner 5e+02))
      (Utilities|IsValid _zombie
        (:Is%20Valid
          (EventDispatchers|BindEventtoOnDead (Actor|GetComponentbyClass _zombie "/Game/Components/Health_component.Health_component_C") (delegate Custom|OnZombieDead))
          (bind _result (Math|Integer|IncrementInt (Variables|Default|GetMobCount))
            (:%20%20
              (Variables|Default|SetMobCount _result))))
        (:Is%20Not%20Valid
          (CallFunction|TrySpawnMob))))))

(event Custom|OnZombieDead
  (bind _result (Math|Integer|DecrementInt (Variables|Default|GetMobCount))
    (:%20%20
      (Variables|Default|SetMobCount _result))))

(event EventBeginPlay
  (bind _box (Variables|Default|GetBox))
  (Collision|AssignOnComponentEndOverlap _box (delegate Custom|OnComponentEndOverlap_Event))
  (Collision|BindEventtoOnComponentBeginOverlap _box (delegate Custom|OnBeginOverlap))
  (Utilities|Time|SetTimerbyEvent (delegate Custom|TrySpawnMob) 1e+01 true true))

(fn ConstructionScript)